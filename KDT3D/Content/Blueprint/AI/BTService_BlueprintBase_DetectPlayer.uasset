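; Behavior tree service that detects a visible BasicCharacter for an AI pawn and publishes it to the blackboard.
; On search start and each tick, it scans the pawn's AIPerceptionComponent for sight-perceived actors.
; The first successful cast to BasicCharacter is stored in the DetectedPlayer key; with no match, the key is set to empty.
; Each tick also prints a debug string.
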(event EventReceiveTickAI
  (params (OwnerController :type AI%20Controller%20Object%20Reference) (ControlledPawn :type Pawn%20Object%20Reference) (DeltaSeconds :type Float%20%28single-precision%29))
  (Development|PrintString "Service" true true "(R=0.566651,G=1.000000,B=0.093511,A=1.000000)")
  (Variables|Default|SetbFound false)
  (bind _array_element (Utilities|Array|ForEachLoopwithBreak (Class|AIPerceptionComponent|GetCurrentlyPerceivedActors (Actor|GetComponentbyClass ControlledPawn "/Script/AIModule.AIPerceptionComponent") "/Script/AIModule.AISense_Sight") :!label _label)
    (:LoopBody
      (bind _asbasic_character (Utilities|Casting|CastToBasicCharacter _array_element))
      (Variables|Default|SetbFound true)
      (AI|Components|Blackboard|SetValueasObject (AI|GetBlackboard OwnerController) (Utilities|Name|MakeLiteralName "DetectedPlayer") _asbasic_character)
      (goto _label Break))
    (:Completed
      (if (not (Variables|Default|GetbFound))
        (AI|Components|Blackboard|SetValueasObject (AI|GetBlackboard (stale EventReceiveSearchStartAI OwnerController)) (Utilities|Name|MakeLiteralName "DetectedPlayer") 0)))))

(event EventReceiveSearchStartAI
  (params (OwnerController :type AI%20Controller%20Object%20Reference) (ControlledPawn :type Pawn%20Object%20Reference))
  (bind _returnvalue (AI|GetBlackboard OwnerController))
  (bind _returnvalue_2 (Utilities|Name|MakeLiteralName "DetectedPlayer"))
  (Variables|Default|SetbFound false)
  (bind _array_element (Utilities|Array|ForEachLoopwithBreak (Class|AIPerceptionComponent|GetCurrentlyPerceivedActors (Actor|GetComponentbyClass ControlledPawn "/Script/AIModule.AIPerceptionComponent") "/Script/AIModule.AISense_Sight") :!label _label)
    (:LoopBody
      (bind _asbasic_character (Utilities|Casting|CastToBasicCharacter _array_element))
      (Variables|Default|SetbFound true)
      (AI|Components|Blackboard|SetValueasObject _returnvalue _returnvalue_2 _asbasic_character)
      (goto _label Break))
    (:Completed
      (if (not (Variables|Default|GetbFound))
        (AI|Components|Blackboard|SetValueasObject _returnvalue _returnvalue_2 0)))))