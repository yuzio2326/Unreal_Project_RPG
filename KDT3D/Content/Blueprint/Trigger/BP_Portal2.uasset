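; Portal trigger that either opens a linked level or, when none is set, teleports the triggering actor to a target transform within the map.
; Teleported pawns also have their control yaw aligned to the destination.
; Activation plays a slowed blink timeline driving emissive power on a dynamic material instance, and deactivation stops it and zeroes the glow.
; The construction script creates that material and labels two text components with the level's short name.
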(event EventBeginPlay
  (Components|Timeline|SetPlayRate (Variables|Default|GetPortalBlinkEffect) 0.4))

(event EventOnActive
  (params (OverlappedComponent :type Primitive%20Component%20Object%20Reference) (OtherActor :type Actor%20Object%20Reference) (OtherComp :type Primitive%20Component%20Object%20Reference) (OtherBodyIndex :type Integer) (bFromSweep :type Boolean) (SweepResult :type Hit%20Result%20Structure%20%28by%20ref%29))
  (bind _power (Timeline|PortalBlinkEffect PlayFromStart)
    (:Update
      (Rendering|Material|SetScalarParameterValue (Variables|디폴트|GetMID) "EmissivePower" (* _power 2e+01) :!class /Script/Engine.MaterialInstanceDynamic))))

(event EventOnTrigger
  (params (OverlappedComponent :type Primitive%20Component%20Object%20Reference) (OtherActor :type Actor%20Object%20Reference) (OtherComp :type Primitive%20Component%20Object%20Reference) (OtherBodyIndex :type Integer) (bFromSweep :type Boolean) (SweepResult :type Hit%20Result%20Structure%20%28by%20ref%29))
  (bind _teleportlocationandrotation (Variables|Default|GetTeleportLocationAndRotation))
  (bind _returnvalue (Transformation|GetWorldRotation _teleportlocationandrotation))
  (if (Utilities|IsValidSoftObjectReference (Variables|Default|GetOpenLevel))
    (Game|OpenLevel(byObjectReference) (Variables|Default|GetOpenLevel))
    (else
      (Transformation|SetActorLocationAndRotation OtherActor (Transformation|GetWorldLocation _teleportlocationandrotation) _returnvalue false true)
      (bind _as폰 (Utilities|Casting|CastToPawn OtherActor))
      (Pawn|SetControlRotation (Pawn|GetController _as폰) (Math|Rotator|MakeRotator (.roll (Pawn|GetControlRotation (Pawn|GetController _as폰) :!class /Script/Engine.Controller)) (.pitch (Pawn|GetControlRotation (Pawn|GetController _as폰) :!class /Script/Engine.Controller)) (.Yaw (Math|Rotator|BreakRotator _returnvalue)))))))

(event EventOnDeactive
  (params (OverlappedComponent :type Primitive%20Component%20Object%20Reference) (OtherActor :type Actor%20Object%20Reference) (OtherComp :type Primitive%20Component%20Object%20Reference) (OtherBodyIndex :type Integer))
  (bind _mid (Variables|디폴트|GetMID))
  (Utilities|FlowControl|Sequence
    (:then_0
      (bind _power (Timeline|PortalBlinkEffect Stop)
        (:Update
          (Rendering|Material|SetScalarParameterValue _mid "EmissivePower" (* _power 2e+01) :!class /Script/Engine.MaterialInstanceDynamic))))
    (:then_1
      (Rendering|Material|SetScalarParameterValue _mid "EmissivePower" 0.0 :!class /Script/Engine.MaterialInstanceDynamic))))

(fn ConstructionScript
  (bind _openlevel (Variables|Default|GetOpenLevel))
  (bind _returnvalue (Utilities|ToString(SoftObjectReference) _openlevel))
  (bind _returnvalue_2 (Utilities|String|FindSubstring _returnvalue "." false true))
  (bind _returnvalue_3 (Utilities|String|Len _returnvalue))
  (bind _returnvalue_4 (+ _returnvalue_2 1))
  (bind _returnvalue_5 (Utilities|String|GetSubstring _returnvalue _returnvalue_4 _returnvalue_3))
  (bind _returnvalue_6 (Utilities|Text|ToText(String) _returnvalue_5))
  (Utilities|FlowControl|Sequence
    (:then_0
      (bind _returnvalue_7 (Rendering|Material|CreateDynamicMaterialInstance (Variables|Default|GetPortalEffect) 0 0 "None" :!class /Script/Engine.PrimitiveComponent))
      (bind _output_get (Variables|디폴트|SetMID _returnvalue_7))
      (Rendering|Material|SetScalarParameterValue _output_get "EmissivePower" 0.0 :!class /Script/Engine.MaterialInstanceDynamic))
    (:then_1
      (if true
        (Rendering|Components|TextRender|SetText (Variables|Default|GetOpenLevelName1) _returnvalue_6)
        (Rendering|Components|TextRender|SetText (Variables|Default|GetOpenLevelName) _returnvalue_6)))))