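; Earth actor for a solar system scene that animates the planet, its cloud layer and an orbiting Moon.
; Every Tick applies frame-time-scaled local yaw rotations, spinning the Earth mesh and counter-rotating the Cloud component at the same speed.
; The Moon spins on its own axis while a separate MoonRotatingAxis component turns more slowly as the pivot for its orbit.
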(event EventBeginPlay)

(event Collision|EventActorBeginOverlap
  (params (OtherActor :type Actor%20Object%20Reference)))

(event EventTick
  (params (DeltaSeconds :type Float%20%28single-precision%29))
  (bind _returnvalue (Utilities|Time|GetWorldDeltaSeconds))
  (Utilities|FlowControl|Sequence
    (:then_0
      ;[1 1 1] 지구 회전
      (Transformation|AddLocalRotation (Variables|Default|GetStaticMesh) (Math|Rotator|MakeRotator 0.0 0.0 (* DeltaSeconds 45.0)) false false)
      (Transformation|AddLocalRotation (Variables|Default|GetCloud) (Math|Rotator|MakeRotator 0.0 0.0 (* (Utilities|Time|GetWorldDeltaSeconds) -45.0)) false false))
    (:then_1
      (Transformation|AddLocalRotation (Variables|Default|GetMoon) (Math|Rotator|MakeRotator 0.0 0.0 (* _returnvalue 1.8e+02)) false false)
      (Transformation|AddLocalRotation (Variables|Default|GetMoonRotatingAxis) (Math|Rotator|MakeRotator 0.0 0.0 (* _returnvalue 6e+01)) false false))))

(fn ConstructionScript)