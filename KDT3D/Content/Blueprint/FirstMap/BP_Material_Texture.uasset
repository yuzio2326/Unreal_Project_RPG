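; BP_Material_Texture is an actor that continuously scrolls the texture on its static mesh's material.
; The construction script creates a dynamic material instance on slot 0 and sets its UV vector parameter from the UV variable.
; Each Tick advances UV's red channel at a fixed rate scaled by delta time and writes it back to that parameter, with no wrapping.
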(event EventBeginPlay)

(event Collision|EventActorBeginOverlap
  (params (OtherActor :type Actor%20Object%20Reference)))

(event EventTick
  (params (DeltaSeconds :type Float%20%28single-precision%29))
  (bind _as머티리얼_인스턴스_다이내믹 (Utilities|Casting|CastToMaterialInstanceDynamic (Rendering|Material|GetMaterial (Variables|Default|GetStaticMesh) 0)))
  (bind _output_get (Variables|Material|SetUV (Utilities|Struct|MakeLinearColor (+ (.r (Variables|Material|GetUV)) (* DeltaSeconds 0.4)) (.g (Variables|Material|GetUV)) (.b (Variables|Material|GetUV)) (.a (Variables|Material|GetUV)))))
  (Rendering|Material|SetVectorParameterValue _as머티리얼_인스턴스_다이내믹 "UV" _output_get :!class /Script/Engine.MaterialInstanceDynamic))

(fn ConstructionScript
  (bind _returnvalue (Rendering|Material|CreateDynamicMaterialInstance (Variables|Default|GetStaticMesh) 0 0 "None" :!class /Script/Engine.PrimitiveComponent))
  (Rendering|Material|SetVectorParameterValue _returnvalue "UV" (Variables|Material|GetUV) :!class /Script/Engine.MaterialInstanceDynamic))