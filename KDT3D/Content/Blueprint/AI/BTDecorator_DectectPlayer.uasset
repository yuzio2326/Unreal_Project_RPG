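; Behavior tree decorator that passes when the AI pawn currently sees a BasicCharacter.
; Its condition check scans the actors its AIPerceptionComponent perceives by sight and casts each to BasicCharacter.
; A match is written to the DetectedPlayer blackboard key, which is cleared when none is found, so the check also updates blackboard state.
; Execution start and finish events only print debug strings.
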(event EventReceiveExecutionFinishAI
  (params (OwnerController :type AI%20Controller%20Object%20Reference) (ControlledPawn :type Pawn%20Object%20Reference) (NodeResult :type EBTNodeResult%20Enum :default "Succeeded"))
  (Development|PrintString "End"))

(event EventReceiveExecutionStartAI
  (params (OwnerController :type AI%20Controller%20Object%20Reference) (ControlledPawn :type Pawn%20Object%20Reference))
  (Development|PrintString "Start"))

(fn PerformConditionCheckAI
  (params (OwnerController :type AI%20Controller%20Object%20Reference) (ControlledPawn :type Pawn%20Object%20Reference))
  (bind _returnvalue (Utilities|Name|MakeLiteralName "DetectedPlayer"))
  (bind _returnvalue_2 (AI|GetBlackboard OwnerController))
  (for _array_element (Class|AIPerceptionComponent|GetCurrentlyPerceivedActors (Actor|GetComponentbyClass ControlledPawn "/Script/AIModule.AIPerceptionComponent") "/Script/AIModule.AISense_Sight")
    (bind _asbasic_character (Utilities|Casting|CastToBasicCharacter _array_element))
    (LocalVariables|SetbFound true)
    (AI|Components|Blackboard|SetValueasObject _returnvalue_2 _returnvalue _asbasic_character))
  (if (LocalVariables|GetbFound)
    _
    (else
      (AI|Components|Blackboard|SetValueasObject _returnvalue_2 _returnvalue 0)))
  (return (LocalVariables|GetbFound)))