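; BPGS_Coin is the coin map's game state, which tracks the coins left and ends the level when all are gone.
; On BeginPlay it counts every BP_Coin actor and binds to each one's OnDestroyed event.
; Each destruction decrements the count; at zero it calls the OnGameClear dispatcher, waits briefly, then opens the lobby map.
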(event Custom|OnCoinDestroyed
  (params (DestroyedActor :type Actor%20Object%20Reference))
  (bind _result (Math|Integer|DecrementInt (Variables|Default|GetRemainCoin))
    (:%20%20
      (if (== _result 0)
        (Default|CallOnGameClear)
        (Utilities|FlowControl|Delay 2.0)
        (Game|OpenLevel(byObjectReference) "/Game/Level/LobbyMap.LobbyMap")))))

(event EventBeginPlay
  (bind _outactors (Actor|GetAllActorsOfClass "/Game/Blueprint/CoinMap/BP_Coin.BP_Coin_C"))
  (Game|BindEventtoOnDestroyed _outactors (delegate Custom|OnCoinDestroyed))
  (Variables|Default|SetRemainCoin (Utilities|Array|Length _outactors)))

(fn ConstructionScript)