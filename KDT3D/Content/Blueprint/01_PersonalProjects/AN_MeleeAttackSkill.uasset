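; Anim notify that deals melee and skill damage from the owning character at the moment it fires.
; The SkillComponent's CurrentAnimIndex selects a scaling of the status component's DMG, replaced by plain DMG when no skill is active.
; During skills, the index also picks a large sphere trace at the GroundEffect or Radiant socket; otherwise a smaller one runs at Weapon.
; Every multi-trace hit receives point damage, with debug drawing left on.
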(fn ReceivedNotify
  (params (MeshComp :type Skeletal%20Mesh%20Component%20Object%20Reference) (Animation :type Anim%20Sequence%20Base%20Object%20Reference) (EventReference :type Anim%20Notify%20Event%20Reference%20Structure%20%28by%20ref%29))
  (bind _returnvalue (Transformation|GetSocketLocation MeshComp "Weapon"))
  (bind _returnvalue_2 (Transformation|GetSocketLocation MeshComp "GroundEffect"))
  (bind _returnvalue_3 (Transformation|GetSocketLocation MeshComp "Radiant"))
  (bind _returnvalue_4 (Components|GetOwner MeshComp))
  (bind _returnvalue_5 (Actor|GetComponentbyClass _returnvalue_4 "/Script/KDT3D.SkillComponent"))
  (bind _returnvalue_6 (Actor|GetComponentbyClass _returnvalue_4 "/Script/KDT3D.CustomDioStatusComponent"))
  (bind _array (Utilities|Array|MakeArray _returnvalue_4))
  (bind _currentanimindex (Variables|/Script/KDT3D.SkillComponent|GetCurrentAnimIndex _returnvalue_5))
  (bind _dmg (Variables|/Script/KDT3D.CustomDioStatusComponent|GetDMG _returnvalue_6))
  (switch int _currentanimindex
    (:0
      (LocalVariables|SetDMGPower 0.0))
    (:1
      (LocalVariables|SetDMGPower (* _dmg 3.0)))
    (:2
      (LocalVariables|SetDMGPower (* _dmg 2.0)))
    (:3
      (LocalVariables|SetDMGPower (+ (* _dmg 1e+01) 3e+02)))
    (:4
      (LocalVariables|SetDMGPower (+ (* _dmg 1e+01) 2.5e+02)))
    (:5
      (LocalVariables|SetDMGPower (+ (* _dmg 15.0) 2e+02)))
    (:6
      (LocalVariables|SetDMGPower (+ (* _dmg 2.5) 87.5)))
    (:7
      (LocalVariables|SetDMGPower (+ (* _dmg 2e+01) 4e+02))))
  (if (Variables|/Script/KDT3D.SkillComponent|GetUsingSkill _returnvalue_5)
    (if (or (== _currentanimindex 4) (or (== _currentanimindex 1) (== _currentanimindex 3)))
      (bind _outhits (Class|KismetSystemLibrary|SphereTraceMultibyProfile _returnvalue_2 _returnvalue_2 3e+02 "Player" false _array "ForDuration" true "(R=1.000000,G=0.000000,B=0.000000,A=1.000000)" "(R=0.000000,G=1.000000,B=0.000000,A=1.000000)" 0.1))
      (bind _as폰 (Utilities|Casting|CastToPawn _returnvalue_4))
      (for _array_element _outhits
        (Game|Damage|ApplyPointDamage (.HitActor (Collision|BreakHitResult _array_element)) (LocalVariables|GetDMGPower) (Math|Vector|VectorZero) _array_element (Pawn|GetController _as폰) _returnvalue_4))
      (elif (or (== _currentanimindex 7) (== _currentanimindex 5))
        (bind _outhits_2 (Class|KismetSystemLibrary|SphereTraceMultibyProfile _returnvalue_3 _returnvalue_3 3e+02 "Player" false _array "ForDuration" true "(R=1.000000,G=0.000000,B=0.000000,A=1.000000)" "(R=0.000000,G=1.000000,B=0.000000,A=1.000000)" 0.1))
        (bind _as폰_2 (Utilities|Casting|CastToPawn _returnvalue_4))
        (for _array_element_2 _outhits_2
          (Game|Damage|ApplyPointDamage (.HitActor (Collision|BreakHitResult _array_element_2)) (LocalVariables|GetDMGPower) (Math|Vector|VectorZero) _array_element_2 (Pawn|GetController _as폰_2) _returnvalue_4))
        (else
          (bind _outhits_3 (Class|KismetSystemLibrary|SphereTraceMultibyProfile _returnvalue _returnvalue 1e+02 "Player" false _array "ForDuration" true "(R=1.000000,G=0.000000,B=0.000000,A=1.000000)" "(R=0.000000,G=1.000000,B=0.000000,A=1.000000)" 0.1 :!label _label))
          (bind _as폰_3 (Utilities|Casting|CastToPawn _returnvalue_4))
          (for _array_element_3 _outhits_3
            (Game|Damage|ApplyPointDamage (.HitActor (Collision|BreakHitResult _array_element_3)) (LocalVariables|GetDMGPower) (Math|Vector|VectorZero) _array_element_3 (Pawn|GetController _as폰_3) _returnvalue_4)))))
    (else
      (LocalVariables|SetDMGPower _dmg)
      (goto _label)))
  (return false))