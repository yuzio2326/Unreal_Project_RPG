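; Player controller for the TPS map that handles item pickup and camera zoom for the controlled pawn.
; On BeginPlay it adds the item and TPS input mapping contexts and sets the SoftWheelSpringArm length limits, which the zoom input switches between.
; Item overlap handlers maintain an array of nearby actors and add or remove a HUD description.
; Pickup destroys the first overlapped actor and calls OnEquipWeapon on BP_TPSCharacter.
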(event Custom|OnEndItemOverlapped
  (params (NewParam :type Actor%20Object%20Reference))
  (Utilities|Array|RemoveItem (Variables|Default|GetOverlappedActors) NewParam)
  (bind _asbp_tpshud (Utilities|Casting|CastToBP_TPSHUD (HUD|GetHUD)))
  (Default|RemoveSimpleItemDesc _asbp_tpshud))

(event Custom|OnBeginItemOverlapped
  (params (NewParam :type Actor%20Object%20Reference))
  (Utilities|Array|Add (Variables|Default|GetOverlappedActors) NewParam)
  (bind _asbp_tpshud (Utilities|Casting|CastToBP_TPSHUD (HUD|GetHUD)))
  (Default|AddSimpleItemDesc _asbp_tpshud))

(event Input|EnhancedActionEvents|EnhancedInputActionIA_PickupItem
  (params (ActionValue :type Boolean) (ElapsedSeconds :type Float%20%28double-precision%29) (TriggeredSeconds :type Float%20%28double-precision%29) (InputAction :type Input%20Action%20Object%20Reference :default "/Game/Blueprint/TPSMap/Input/Item/IA_PickupItem.IA_PickupItem"))
  (bind _overlappedactors (Variables|Default|GetOverlappedActors))
  (:Started
    (if (Utilities|Array|IsNotEmpty _overlappedactors)
      (Actor|DestroyActor (Utilities|Array|Get(acopy) _overlappedactors))
      (bind _asbp_tpscharacter (Utilities|Casting|CastToBP_TPSCharacter (Pawn|GetControlledPawn)))
      (Default|OnEquipWeapon _asbp_tpscharacter))))

(event Input|EnhancedActionEvents|EnhancedInputActionIA_Zoom
  (params (ActionValue :type Boolean) (ElapsedSeconds :type Float%20%28double-precision%29) (TriggeredSeconds :type Float%20%28double-precision%29) (InputAction :type Input%20Action%20Object%20Reference :default "/Game/Blueprint/TPSMap/Input/TPS/IA_Zoom.IA_Zoom"))
  (bind _returnvalue (Pawn|GetControlledPawn))
  (bind _returnvalue_2 (Actor|GetComponentbyClass _returnvalue "/Script/KDT3D.SoftWheelSpringArmComponent"))
  (:Started
    (Class|SoftWheelSpringArmComponent|SetDesiredZoom _returnvalue_2 1e+02))
  (:Completed
    (Class|SoftWheelSpringArmComponent|SetDesiredZoom _returnvalue_2 2.5e+02)))

(event EventBeginPlay
  (bind _returnvalue (PlayerController|LocalPlayerSubsystems|GetEnhancedInputLocalPlayerSubsystem))
  (Input|AddMappingContext _returnvalue "/Game/Blueprint/TPSMap/Input/Item/IMC_Item.IMC_Item" 0 "(bIgnoreAllPressedKeysUntilRelease=True,bForceImmediately=False,bNotifyUserSettings=False)")
  (Input|AddMappingContext _returnvalue "/Game/Blueprint/TPSMap/Input/TPS/IMC_TPS.IMC_TPS" 0 "(bIgnoreAllPressedKeysUntilRelease=True,bForceImmediately=False,bNotifyUserSettings=False)")
  (Class|SoftWheelSpringArmComponent|SetMinMaxTargetArmLength (Actor|GetComponentbyClass (Pawn|GetControlledPawn) "/Script/KDT3D.SoftWheelSpringArmComponent") 1e+02 2.5e+02))

(event EventTick
  (params (DeltaSeconds :type Float%20%28single-precision%29)))

(fn ConstructionScript)