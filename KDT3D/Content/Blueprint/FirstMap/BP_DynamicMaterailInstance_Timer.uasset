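; Demo actor that cycles the BaseColor parameter of a dynamic material instance through red, green and blue on a timer.
; BeginPlay starts a looping two-second timer bound to a custom event.
; That event drives a looping, in-order MultiGate, with each output setting the next color on the MID variable, which these graphs never create or assign.
; Tick only calls its parent, and a leftover world-offset node never runs.
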(event Custom|TimerEvent
  (bind _mid (Variables|Default|GetMID))
  (Utilities|FlowControl|MultiGate false true -1
    (:Out%200
      (Rendering|Material|SetVectorParameterValue _mid "BaseColor" "(R=1.000000,G=0.000000,B=0.000000,A=1.000000)" :!class /Script/Engine.MaterialInstanceDynamic))
    (:Out%201
      (Rendering|Material|SetVectorParameterValue _mid "BaseColor" "(R=0.024615,G=1.000000,B=0.000000,A=1.000000)" :!class /Script/Engine.MaterialInstanceDynamic))
    (:Out%202
      (Rendering|Material|SetVectorParameterValue _mid "BaseColor" "(R=0.000000,G=0.178259,B=1.000000,A=1.000000)" :!class /Script/Engine.MaterialInstanceDynamic))))

(event EventBeginPlay
  (|CallParentFunction)
  (Utilities|Time|SetTimerbyEvent (delegate Custom|TimerEvent) 2.0 true))

(event EventTick
  (params (DeltaSeconds :type Float%20%28single-precision%29))
  (|CallParentFunction DeltaSeconds))

(fn ConstructionScript
  (|CallParentFunction))