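; Behavior tree task that walks the controlled pawn along the points of a spline, one point per execution.
; It reads the spline from the SplineComponent blackboard key, increments a point index wrapped by the point count, and runs AI MoveTo to that point's world location.
; The task finishes as successful whether the move succeeds or fails, but never finishes if the spline cast fails.
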(event EventReceiveExecuteAI
  (params (OwnerController :type AI%20Controller%20Object%20Reference) (ControlledPawn :type Pawn%20Object%20Reference))
  (bind _as스플라인_컴포넌트 (Utilities|Casting|CastToSplineComponent (AI|Components|Blackboard|GetValueasObject (AI|GetBlackboard OwnerController) (Utilities|Name|MakeLiteralName "SplineComponent"))))
  (bind _output_get (Variables|Default|SetSplineComponent _as스플라인_컴포넌트))
  (bind _output_get_2 (Variables|Default|SetMaxPointIndex (Spline|GetNumberOfSplinePoints _output_get)))
  (bind _result (Math|Integer|IncrementInt (Variables|Default|GetPointIndex))
    (:%20%20
      (bind _output_get_3 (Variables|Default|SetPointIndex (Math|Integer|%(Integer) _result _output_get_2)))
      (AI|AIMoveTo ControlledPawn (Spline|GetLocationatSplinePoint (Variables|Default|GetSplineComponent) _output_get_3 "World") 0 5.0 false
        (:OnSuccess
          _)
        (:OnFail
          _))
      (AI|BehaviorTree|FinishExecute true))))

(event EventReceiveTickAI
  (params (OwnerController :type AI%20Controller%20Object%20Reference) (ControlledPawn :type Pawn%20Object%20Reference) (DeltaSeconds :type Float%20%28single-precision%29)))